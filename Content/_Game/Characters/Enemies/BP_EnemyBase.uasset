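; BP_EnemyBase is the base enemy character Blueprint, supplying motion-warp facing and dissolve effects.
; UpdateFacingTarget sets a "FacingTarget" warp target at a given location on the MotionWarping component.
; Two events store a passed-in dynamic material instance, one for the body and one for the weapon, then play separate timelines that drive each material's "Dissolve" scalar parameter.
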(event `CombatInterface.UpdateFacingTarget`
  (params (TargetLocation :type "Vector Structure (by ref)"))
  (`MotionWarpingComponent.AddOrUpdateWarpTargetFromLocation` (`self.MotionWarping`) "FacingTarget" TargetLocation))

(event `self.StartDissolveTimeline`
  (params (DynamicMaterialInstance :type "MaterialInstanceDynamic Object Reference"))
  (set `self.DynamicMaterialInstance` DynamicMaterialInstance)
  (bind (_direction _dissolvetrack) (`Timeline|DissolveTimeline`)
    (:`Update`
      (`MaterialInstanceDynamic.SetScalarParameterValue` (`self.DynamicMaterialInstance`) "Dissolve" _dissolvetrack))))

(event `self.StartWeaponDissolveTimeline`
  (params (DynamicMaterialInstance :type "MaterialInstanceDynamic Object Reference"))
  (set `self.WeaponDynamicMaterialInstance` DynamicMaterialInstance)
  (bind (_direction _weapondissolvetrack) (`Timeline|WeaponDissolveTimeline`)
    (:`Update`
      (`MaterialInstanceDynamic.SetScalarParameterValue` (`self.WeaponDynamicMaterialInstance`) "Dissolve" _weapondissolvetrack))))

(fn `UserConstructionScript`)