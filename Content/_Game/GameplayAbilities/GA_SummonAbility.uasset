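; Gameplay ability that summons random minions around its avatar, likely the shaman enemy, at locations it computes.
; On activation it shuffles the spawn points, shows a ground summon effect at each and plays the summon montage.
; A montage gameplay event starts a delayed loop spawning one AI-controlled minion per point, facing away from the avatar.
; The avatar's minion count rises on each spawn and falls when a minion is destroyed.
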(event `self.K2_ActivateAbility`
  (bind _spawnlocationindex (`self.SpawnLocationIndex`))
  (bind _spawnlocations (`self.SpawnLocations`))
  (bind _returnvalue (+ (`|GetArrayItem` _spawnlocations _spawnlocationindex) (`self.SpawnVector`)))
  (set `self.AvatarActorFromActorInfo` (`self.GetAvatarActorFromActorInfo`))
  (bind _returnvalue_2 (`self.GetSpawnLocations`))
  (bind _output_get (set `self.SpawnLocations` _returnvalue_2))
  (`KismetArrayLibrary.Array_Shuffle` _output_get)
  (for _array_element (`self.SpawnLocations`)
    (`NiagaraFunctionLibrary.SpawnSystemAtLocation` "/Game/Assets/Effects/Combat/NS_GroundSummon.NS_GroundSummon" _array_element))
  (`AbilityTask_PlayMontageAndWait.CreatePlayMontageAndWaitProxy` "None" "/Game/_Game/Characters/Enemies/Shaman/Animations/AM_Summon_Shaman.AM_Summon_Shaman"
    (:`then`
      (`AbilityTask_WaitGameplayEvent.WaitGameplayEvent` (struct :`TagName` "Montage.Attack.1") null
        (:`EventReceived`
          (if (< _spawnlocationindex (`KismetArrayLibrary.Array_Length` _spawnlocations)) :!label _label
            (bind _returnvalue_3 (`|SpawnActorFromClass` (`self.GetRandomMinionClass`) (`KismetMathLibrary.MakeTransform` _returnvalue (`KismetMathLibrary.FindLookAtRotation` (`Actor.K2_GetActorLocation` (`self.AvatarActorFromActorInfo`)) _returnvalue)) "AlwaysSpawn" "MultiplyWithRoot" null null))
            (bind _output_get_2 (set `self.MinionPawn` _returnvalue_3))
            (add `Actor.OnDestroyed` _output_get_2 (delegate `OnDestroyed`))
            (`Pawn.SpawnDefaultController` (`self.MinionPawn`))
            (message `CombatInterface.IncrementMinionCount` (`self.AvatarActorFromActorInfo`) 1)
            (`/Engine/EditorBlueprintResources/StandardMacros.IncrementInt` (`self.SpawnLocationIndex`)
              (:`  `
                (`KismetSystemLibrary.Delay` 0.1)
                (goto _label)))))))))

(event `OnDestroyed`
  (params (DestroyedActor :type "Actor Object Reference"))
  (message `CombatInterface.DecrementMinionCount` (`self.AvatarActorFromActorInfo`) 1))