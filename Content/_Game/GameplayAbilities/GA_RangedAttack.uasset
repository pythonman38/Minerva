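; Gameplay ability for a ranged attack that turns the avatar toward its combat target and fires a projectile at it.
; It plays a random tagged montage from the avatar's attack set and waits for a gameplay event matching that montage's tag.
; On the event it re-reads the target's location, calls SpawnProjectile and ends; montage completion, interruption or cancellation also ends it.
; Avatar data comes through interface messages.
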(event `self.K2_ActivateAbility`
  (bind _avataractorfromactorinfo (`self.AvatarActorFromActorInfo`))
  (bind _avataractorfromactorinfo_2 (`self.AvatarActorFromActorInfo`))
  (bind _output_get (set `self.AvatarActorFromActorInfo` (`self.GetAvatarActorFromActorInfo`)))
  (bind _returnvalue (message `EnemyInterface.GetCombatTarget` _output_get))
  (message `CombatInterface.UpdateFacingTarget` _avataractorfromactorinfo (`Actor.K2_GetActorLocation` _returnvalue))
  (bind _returnvalue_2 (message `CombatInterface.GetAttackMontages` _avataractorfromactorinfo))
  (bind _output_get_2 (set `self.TaggedMontage` (`self.GetRandomTaggedMontageFromArray` _returnvalue_2)))
  (`AbilityTask_PlayMontageAndWait.CreatePlayMontageAndWaitProxy` "None" (break `TaggedMontage` _output_get_2) 1.0 "None" false
    (:`then`
      (`AbilityTask_WaitGameplayEvent.WaitGameplayEvent` (`.MontageTag` (break `TaggedMontage` _output_get_2)) null
        (:`EventReceived`
          (message `CombatInterface.GetCombatSocketLocation` _avataractorfromactorinfo_2 (`.MontageTag` (break `TaggedMontage` _output_get_2)))
          (bind _returnvalue_3 (message `EnemyInterface.GetCombatTarget` _avataractorfromactorinfo_2))
          (`self.SpawnProjectile` (`Actor.K2_GetActorLocation` _returnvalue_3))
          (`self.K2_EndAbility`))))
    (:`OnCompleted`
      (`self.K2_EndAbility` :!label _label))
    (:`OnInterrupted`
      (goto _label))
    (:`OnCancelled`
      (goto _label))))