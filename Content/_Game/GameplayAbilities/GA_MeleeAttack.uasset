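; Melee attack gameplay ability that turns the avatar toward its combat target and plays a random tagged attack montage.
; On the montage's gameplay event, it damages non-friendly live players near the tagged combat socket and triggers their blood effect.
; Any hit fires a MeleeImpact cue carrying the montage tag.
; The ability ends after that event or when the montage finishes or is interrupted, without stopping the montage.
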(event `self.K2_ActivateAbility`
  (bind _returnvalue (`self.GetAvatarActorFromActorInfo`))
  (bind _avataractorfromactorinfo (`self.AvatarActorFromActorInfo`))
  (bind _avataractorfromactorinfo_2 (`self.AvatarActorFromActorInfo`))
  (bind (_taggedmontage_montage _taggedmontage_montagetag) (break `TaggedMontage` (`self.TaggedMontage`)))
  (set `self.HasHitTarget` false)
  (bind _output_get (set `self.AvatarActorFromActorInfo` _returnvalue))
  (bind _returnvalue_2 (message `EnemyInterface.GetCombatTarget` _output_get))
  (bind _ascombat_interface (cast `CombatInterface` _returnvalue))
  (`CombatInterface.UpdateFacingTarget` _ascombat_interface (`Actor.K2_GetActorLocation` _returnvalue_2))
  (bind _returnvalue_3 (message `CombatInterface.GetAttackMontages` (`self.AvatarActorFromActorInfo`)))
  (bind _output_get_2 (set `self.TaggedMontage` (`self.GetRandomTaggedMontageFromArray` _returnvalue_3)))
  (`AbilityTask_PlayMontageAndWait.CreatePlayMontageAndWaitProxy` "None" (break `TaggedMontage` _output_get_2) 1.0 "None" false
    (:`then`
      (`AbilityTask_WaitGameplayEvent.WaitGameplayEvent` (`.MontageTag` (break `TaggedMontage` _output_get_2)) null
        (:`EventReceived`
          (bind _returnvalue_4 (message `CombatInterface.GetCombatSocketLocation` _avataractorfromactorinfo (`.SocketTag` (break `TaggedMontage` _output_get_2))))
          (bind _output_get_3 (set `self.CombatSocketLocation` _returnvalue_4))
          (bind _outoverlappingactors (`MinervaAbilitySystemLibrary.GetLivePlayersWithinRadius` _avataractorfromactorinfo (`|MakeArray` _avataractorfromactorinfo) 45.0 _output_get_3))
          (for _array_element _outoverlappingactors
            (bind _output_get_4 (set `self.ArrayElement` _array_element))
            (if (`MinervaAbilitySystemLibrary.IsNotFriend` _avataractorfromactorinfo_2 _array_element)
              (`self.CauseDamage` _output_get_4)
              (set `self.HasHitTarget` true)
              (message `CombatInterface.GetBloodEffect` (`self.ArrayElement`))))
          (if (`self.HasHitTarget`)
            (bind _returnvalue_5 (message `EnemyInterface.GetCombatTarget` _avataractorfromactorinfo_2))
            (`self.K2_ExecuteGameplayCueWithParams` (struct :`TagName` "GameplayCue.MeleeImpact") (`AbilitySystemBlueprintLibrary.MakeGameplayCueParameters` 0.0 0.0 (struct) (struct) (struct) (`BlueprintGameplayTagLibrary.MakeGameplayTagContainerFromTag` _taggedmontage_montagetag) (struct) (`self.CombatSocketLocation`) (0.0 0.0 0.0) null _avataractorfromactorinfo_2 _returnvalue_5)))
          (`self.K2_EndAbility`))))
    (:`OnCompleted`
      (`self.K2_EndAbility` :!label _label))
    (:`OnInterrupted`
      (goto _label))
    (:`OnCancelled`
      (goto _label))))